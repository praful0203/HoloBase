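; BP_HandMenu is a mixed reality hand menu built with UX Tools (UXT) components, shown and hidden by a palm-up gesture.
; The palm-up constraint's activated and deactivated events set the UI element's visibility to Show or Hide.
; Tick polls the UpButton child actor's pressable button state and prints a debug message on every frame it reads Pressed, with no other action attached.
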(event OnConstraintActivated(UxtPalmUpConstraint)
  (Class|UxtUIElementComponent|SetUIVisibility (Variables|Default|GetUxtUIElement) "Show"))

(event OnConstraintDeactivated(UxtPalmUpConstraint)
  (Class|UxtUIElementComponent|SetUIVisibility (Variables|Default|GetUxtUIElement) "Hide"))

(event EventBeginPlay)

(event Collision|EventActorBeginOverlap
  (params (OtherActor :type Actor%20Object%20Reference)))

(event EventTick
  (params (DeltaSeconds :type Float%20%28single-precision%29))
  (bind _asuxt_pressable_button_actor (Utilities|Casting|CastToUxtPressableButtonActor (Variables|/Script/Engine.ChildActorComponent|GetChildActor (Variables|Default|GetUpButton))))
  (if (Utilities|Enum|Equal(Enum) (Class|UxtPressableButtonComponent|GetState (Variables|/Script/UXTools.UxtBasePressableButtonActor|GetButtonComponent _asuxt_pressable_button_actor)) "Pressed")
    (Development|PrintString "Button Pressed")))

(fn ConstructionScript)